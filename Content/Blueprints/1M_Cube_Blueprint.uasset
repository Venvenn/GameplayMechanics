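; Physics-driven cube that drives itself forward at constant speed and is steered by the MotionControllerPawn.
; Each Tick it finds the pawn with GetAllActorsOfClass, copies its veer flags and sets linear velocity along the actor's forward vector.
; Either flag yaws the mesh by a fixed per-frame step and turns the Cylinder alongside it, capped by world-yaw limits.
; Logic to attach the pawn at a "Player" socket is present but never runs.
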(event `self.ReceiveTick`
  (params (DeltaSeconds :type "Float (single-precision)"))
  (bind _staticmeshcomponent (`self.StaticMeshComponent`))
  (bind _cylinder (`self.Cylinder`))
  (bind (_returnvalue_roll _returnvalue_pitch _returnvalue_yaw) (`KismetMathLibrary.BreakRotator` (`SceneComponent.K2_GetComponentRotation` _cylinder)))
  (bind (_returnvalue_roll_2 _returnvalue_pitch_2 _returnvalue_yaw_2) (`KismetMathLibrary.BreakRotator` (`SceneComponent.K2_GetComponentRotation` _cylinder)))
  (bind _roll (.roll (`SceneComponent.K2_GetComponentRotation` _staticmeshcomponent)))
  (bind _pitch (.pitch (`SceneComponent.K2_GetComponentRotation` _staticmeshcomponent)))
  (bind _yaw (.yaw (`SceneComponent.K2_GetComponentRotation` _staticmeshcomponent)))
  (bind _returnvalue (+ _returnvalue_yaw -0.1))
  (bind _returnvalue_2 (+ _returnvalue_yaw_2 0.1))
  (bind _outactors (`GameplayStatics.GetAllActorsOfClass` "/Game/VirtualRealityBP/Blueprints/MotionControllerPawn.MotionControllerPawn_C"))
  (bind _item (`KismetArrayLibrary.Array_Get` _outactors))
  (set `self.VeerLeft` (`/Game/VirtualRealityBP/Blueprints/MotionControllerPawn.VeerL` _item))
  (set `self.VeerRight` (`/Game/VirtualRealityBP/Blueprints/MotionControllerPawn.VeerR` _item))
  (`|ExecutionSequence`
    (:`then_0`
      (`PrimitiveComponent.SetPhysicsLinearVelocity` _staticmeshcomponent (* (`KismetMathLibrary.GetForwardVector` (`self.K2_GetActorRotation`)) 300.0) false "None"))
    (:`then_1`
      (if (`self.VeerRight`)
        (`SceneComponent.K2_SetWorldRotation` _staticmeshcomponent (`KismetMathLibrary.MakeRotator` _roll _pitch (+ _yaw 0.1)) false false)
        (if (not (>= _returnvalue_2 50.0))
          (`SceneComponent.K2_SetWorldRotation` _cylinder (`KismetMathLibrary.MakeRotator` _returnvalue_roll_2 _returnvalue_pitch_2 _returnvalue_2) false false))))
    (:`then_2`
      (if (`self.VeerLeft`)
        (`SceneComponent.K2_SetWorldRotation` _staticmeshcomponent (`KismetMathLibrary.MakeRotator` _roll _pitch (+ _yaw -0.1)) false false)
        (if (not (<= _returnvalue -50.0))
          (`SceneComponent.K2_SetWorldRotation` _cylinder (`KismetMathLibrary.MakeRotator` _returnvalue_roll _returnvalue_pitch _returnvalue) false false))))))

(event `self.ReceiveBeginPlay`)

(fn `UserConstructionScript`)