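; Cannon actor that enables player input and fires CannonBall projectiles from the left motion controller Grip1 or R key.
; Each shot with ammo spawns a ball at LaunchPoint, applies a large force along the actor's forward vector, decrements ammo and starts regeneration.
; Tick adds one ammo after the Regeneration delay, then stops regenerating unless Ammo equals 10, so the cap check appears inverted.
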(event `self.ReceiveBeginPlay`
  (`self.EnableInput` (`GameplayStatics.GetPlayerController` 0) null) ; Make sure Actor is getting input
)

(event `self.ReceiveTick`
  (params (DeltaSeconds :type "Float (single-precision)"))
  (if (`self.regenerating`)
    (set `self.timer` (+ (`self.timer`) DeltaSeconds)) ; Add Delta Time to Timer
    (if (> (`self.timer`) (`self.regeneration`))
      (bind _result (`/Engine/EditorBlueprintResources/StandardMacros.IncrementInt` (`self.ammo`)) ; Incriment Ammo count by one
        (:`  `
          (set `self.ammo` _result)
          (if (== (`self.ammo`) 10)
            (set `self.timer` 0.0)
            (else
              (set `self.regenerating` false)
              (set `self.timer` 0.0))))))))

(event `Key|MotionController_Left_Grip1`
  (params (Key :type "Key Structure" :default "AnyKey"))
  (:`Pressed`
    (if (> (`self.ammo`) 0) :!label _label
      (bind _returnvalue (`|SpawnActorFromClass` "/Game/Blueprints/CannonBall.CannonBall_C" (`SceneComponent.K2_GetComponentToWorld` (`self.LaunchPoint`)) "Undefined" "OverrideRootScale")) ; Change to your Own projectile actor
      (`PrimitiveComponent.AddForce` (`/Game/Blueprints/CannonBall.Sphere` _returnvalue) (* (`KismetMathLibrary.GetForwardVector` (`self.K2_GetActorRotation`)) 30000000.0) "None" false) ; "Launch" it
      (bind _result (`/Engine/EditorBlueprintResources/StandardMacros.DecrementInt` (`self.ammo`)) ; reduce ammo counter
        (:`  `
          (set `self.ammo` _result)
          (set `self.regenerating` true) ; Turn On Regeneration
        )))))

(event `Key|R` :consume false
  (params (Key :type "Key Structure" :default "AnyKey"))
  (:`Pressed`
    (goto _label)))

(fn `UserConstructionScript`)