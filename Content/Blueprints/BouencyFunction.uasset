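; Blueprint buoyancy helpers that push an object up or down at a given local point.
; WaveHight applies a mass-scaled force at that point: upward by Displacement when underwater, otherwise downward at gravity strength, both scaled by Amount.
; EvaluatePointHight derives Amount from a clamped cubic of depth over Thickness.
; Its height inputs are zero vectors, ignoring Manager, Time and the transformed point, so depth is always zero.
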(fn `EvaluatePointHight`
  (params (Location :type "Vector Structure") (Transform :type "Transform Structure") (Manager :type "Actor Object Reference") (Thickness :type "Float (double-precision)") (Time :type "Float (double-precision)"))
  (returns (UnderWater :type Boolean) (Amount :type "Float (double-precision)") (Delta :type "Float (double-precision)") (`Intersect Point` :type "Vector Structure") (Hight :type "Float (double-precision)"))
  (bind _z (.z (0.0 0.0 0.0)))
  (bind _returnvalue (- (.z (0.0 0.0 0.0)) _z))
  (return (> _returnvalue 0.0) (`KismetMathLibrary.Abs` (`KismetMathLibrary.FClamp` (`KismetMathLibrary.MultiplyMultiply_FloatFloat` (/ _returnvalue Thickness) 3.0) -10.0)) _returnvalue (`KismetMathLibrary.MakeVector` (.x (0.0 0.0 0.0)) (.y (0.0 0.0 0.0)) _z) 0.0))

(fn `WaveHight`
  (params (Point :type "Vector Structure") (Object :type "PrimitiveComponent Object Reference") (Manager :type "Actor Object Reference") (Transform :type "Transform Structure") (Mass :type "Float (double-precision)") (thickness :type "Float (double-precision)") (Displacement :type "Float (double-precision)") (Time :type "Float (double-precision)"))
  (bind _returnvalue (`KismetMathLibrary.TransformLocation` Transform Point))
  (bind (_underwater _amount) (`self.EvaluatePointHight` Point Transform Manager thickness Time))
  (if _underwater
    (`PrimitiveComponent.AddForceAtLocation` Object (* (* (`KismetMathLibrary.MakeVector` 0.0 0.0 (* Displacement 980.0)) Mass) _amount) _returnvalue "None")
    (else
      (`PrimitiveComponent.AddForceAtLocation` Object (* (* (`KismetMathLibrary.MakeVector` 0.0 0.0 -980.0) Mass) _amount) _returnvalue "None"))))